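; Base game mode that runs a timed run, with a start delay, HUD timer and respawn point registration.
; On BeginPlay it locks player input, resets the active respawn point, creates the main HUD and assigns each respawn point its array index as SpawnID.
; A delayed event restores input and starts a looping timer feeding CalcTime's real-time clock values to the HUD.
; GameWonStopTimer pauses the clock, hides it and prints the final time.
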(event Custom|GameStartEvent
  ;[0.15 0.15 0.15 0.5] Start Game Timer + Game Timer
  ;;[0.15 0.15 0.15 0.5] Enable inputs & clear timer
  (Input|EnableInput (Game|GetPlayerCharacter 0) 0)
  (Utilities|Time|ClearandInvalidateTimerbyHandle (Variables|Time|GetGameStartTimer))
  ;;[0.15 0.15 0.15 0.5] Save Start Seconds
  (Variables|Time|SetStartSeconds (Math|Conversions|ToFloat(Integer) (.Seconds (Class|GameplayStatics|GetAccurateRealTime))))
  ;;[0.15 0.15 0.15 0.5] Update Timer
  (bind _returnvalue (Utilities|Time|SetTimerbyEvent (delegate Custom|TimerTimerEvent) 0.01 true))
  (Variables|Time|SetTimersTimer _returnvalue))

(event Custom|GameWonStopTimer
  (Utilities|Time|PauseTimerbyHandle (Variables|Time|GetTimersTimer))
  (Widget|SetVisibility (Variables|/Game/Widgets/Game/WBP_MainGameHUD.WBP_MainGameHUD_C|GetWBP_TimeDisplay (Variables|Default|GetMainGameHud)) "Hidden")
  (Development|PrintText (Utilities|Text|FormatText "{a} : {b} : {c}" (Variables|Default|GetTimerMinutes) (Variables|Default|GetTimerSeconds) (Math|Float|Truncate (Variables|Default|GetTimerMS)))))

(event Custom|TimerTimerEvent
  ;[0.15 0.15 0.15 0.5] Start Game Timer + Game Timer
  ;;[0.15 0.15 0.15 0.5] Update Timer
  (bind (_ms _sec _min) (CallFunction|CalcTime))
  (Default|UpdateTimer (Variables|/Game/Widgets/Game/WBP_MainGameHUD.WBP_MainGameHUD_C|GetWBP_TimeDisplay (Variables|Default|GetMainGameHud)) _ms _sec _min))

(event EventBeginPlay
  (bind _returnvalue (Game|GetPlayerController 0))
  ;[0.15 0.15 0.15 0.5] Disable inputs
  (Input|DisableInput (Game|GetPlayerCharacter 0) 0)
  ;[0.15 0.15 0.15 0.5] Clear Respawn Points
  (Variables|/Game/Blueprints/Base/GI_Main.GI_Main_C|SetActiveRespawnPoint (CallFunction|GetGI) 0)
  (Utilities|FlowControl|Sequence
    (:then_0
      ;[0.15 0.15 0.15 0.5] Create widget & set input mode
      (bind _returnvalue_2 (UserInterface|CreateWidget "/Game/Widgets/Game/WBP_MainGameHUD.WBP_MainGameHUD_C"))
      (bind _output_get (Variables|Default|SetMainGameHud _returnvalue_2))
      (UserInterface|Viewport|AddtoViewport _output_get 0)
      (Input|SetInputModeGameOnly _returnvalue false)
      (Variables|/Script/Engine.PlayerController|SetbShowMouseCursor _returnvalue false))
    (:then_1
      ;[0.15 0.15 0.15 0.5] Start Game Timer + Game Timer
      (bind _returnvalue_3 (Utilities|Time|SetTimerbyEvent (delegate Custom|GameStartEvent) 3.0))
      (Variables|Time|SetGameStartTimer _returnvalue_3))
    (:then_2
      (bind _outactors (Actor|GetAllActorsOfClass "/Game/Blueprints/RespawnPoints/BP_RespawnPoints.BP_RespawnPoints_C"))
      (for _array_element _outactors
        (bind _returnvalue_4 (Utilities|Array|Add (Variables|Respawn|GetRespawnPoints) _array_element))
        (Variables|/Game/Blueprints/RespawnPoints/BP_RespawnPoints.BP_RespawnPoints_C|SetSpawnID _array_element _returnvalue_4)))))

(fn ConstructionScript)

(fn CalcTime
  (bind (_seconds _partialseconds) (Class|GameplayStatics|GetAccurateRealTime))
  (bind _output_get (LocalVariables|SetElapsedTime (- _seconds (Variables|Time|GetStartSeconds))))
  (Variables|Default|SetTimerMS (* (Math|Float|%(Float) _partialseconds 1.0) 1e+03))
  (bind _output_get_2 (Variables|Default|SetTimerSeconds (Math|Float|Floor (Math|Float|%(Float) _output_get 6e+01))))
  (bind _output_get_3 (Variables|Default|SetTimerMinutes (Math|Float|Floor (/ _output_get 6e+01))))
  (return (Math|Float|Truncate (Variables|Default|GetTimerMS)) _output_get_2 _output_get_3))