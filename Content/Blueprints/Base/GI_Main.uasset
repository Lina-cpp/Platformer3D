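; Game instance Blueprint that works out which levels come before and after the current one in the game's map list.
; FindGameLevels gets the current level name and stores the next and previous level names, with found flags and debug prints.
; Its helper functions locate the current name in the GameMaps array and step one index forward or back, checking that the index is valid.
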(event Custom|FindGameLevels
  (bind _returnvalue (Game|GetCurrentLevelName true))
  (Utilities|FlowControl|Sequence
    (:then_0
      (bind (_currentlevelfromarray _bisvalidindex) (CallFunction|FindNextLevel _returnvalue))
      (if _bisvalidindex
        (Variables|FindLevel|SetNextLevel _currentlevelfromarray)
        (Variables|FindLevel|SetbWasNextLevelFound true)
        (Development|PrintString "nex lvl found")
        (else
          (Variables|FindLevel|SetbWasNextLevelFound false)
          (Development|PrintString "No next level" true true "(R=1.000000,G=0.000000,B=0.072882,A=1.000000)"))))
    (:then_1
      (bind (_previouslevelname _bisindexvalid) (CallFunction|FindPreviousLevel _returnvalue))
      (if _bisindexvalid
        (Variables|FindLevel|SetPreviousLevel _previouslevelname)
        (Variables|FindLevel|SetbWasPrevLevelFound true)
        (Development|PrintString "prev lvl found")
        (else
          (Variables|FindLevel|SetbWasPrevLevelFound false)
          (Development|PrintString "no prev level" true true "(R=1.000000,G=0.000000,B=0.284335,A=1.000000)"))))))

(fn FindCurrentLevelinArray
  (params (CurrentLevel :type String%20%28by%20ref%29))
  (bind _returnvalue (Utilities|String|StringToName CurrentLevel))
  (bind _gamemaps (Variables|FindLevel|GetGameMaps))
  (bind _returnvalue_2 (Utilities|Array|FindItem _gamemaps _returnvalue))
  (if (Utilities|Array|IsValidIndex _gamemaps _returnvalue_2)
    (return (Utilities|Array|Get(acopy) _gamemaps _returnvalue_2) _returnvalue_2)))

(fn FindNextLevel
  (params (CurrentLevel :type String%20%28by%20ref%29))
  (bind _gamemaps (Variables|FindLevel|GetGameMaps))
  (bind _currentlevelindex (CallFunction|FindCurrentLevelinArray CurrentLevel))
  (if (Utilities|Array|IsValidIndex _gamemaps (+ _currentlevelindex 1))
    (return (Utilities|Array|Get(acopy) _gamemaps (+ _currentlevelindex 1)) (Utilities|Array|IsValidIndex _gamemaps (+ _currentlevelindex 1)))))

(fn FindPreviousLevel
  (params (CurrentLevel :type String%20%28by%20ref%29))
  (bind _gamemaps (Variables|FindLevel|GetGameMaps))
  (bind _currentlevelindex (CallFunction|FindCurrentLevelinArray CurrentLevel))
  (if (Utilities|Array|IsValidIndex _gamemaps (- _currentlevelindex 1))
    (return (Utilities|Array|Get(acopy) _gamemaps (- _currentlevelindex 1)) (Utilities|Array|IsValidIndex _gamemaps (- _currentlevelindex 1)))))