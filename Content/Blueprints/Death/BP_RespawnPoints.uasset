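; BP_RespawnPoints is a checkpoint actor that records itself as the active respawn point and repositions the player there.
; When a BP_PlayerCharacterBase overlaps its Box, it writes its SpawnID to ActiveRespawnPoint on the game instance, skipping living players when already active.
; MovePlayerToRespawnPoint teleports a given player to the RespawnLocation component's position, facing the Arrow's rotation.
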(event OnComponentBeginOverlap(Box)
  (params (OverlappedComponent :type Primitive%20Component%20Object%20Reference) (OtherActor :type Actor%20Object%20Reference) (OtherComp :type Primitive%20Component%20Object%20Reference) (OtherBodyIndex :type Integer) (bFromSweep :type Boolean) (SweepResult :type Hit%20Result%20Structure%20%28by%20ref%29))
  (bind _asgi_main (CallFunction|GetGI))
  (bind _asbp_player_character_base (Utilities|Casting|CastToBP_PlayerCharacterBase OtherActor))
  (if (not (and (not (Variables|/Script/Platformer3D.CharacterBase|GetbIsDead _asbp_player_character_base)) (== (Variables|/Game/Blueprints/Base/GI_Main.GI_Main_C|GetActiveRespawnPoint _asgi_main) (Variables|Default|GetSpawnID))))
    (Variables|/Game/Blueprints/Base/GI_Main.GI_Main_C|SetActiveRespawnPoint _asgi_main (Variables|Default|GetSpawnID))))

(event EventBeginPlay)

(event Collision|EventActorBeginOverlap
  (params (OtherActor :type Actor%20Object%20Reference)))

(event EventTick
  (params (DeltaSeconds :type Float%20%28single-precision%29)))

(fn ConstructionScript)

(fn MovePlayertoRespawnPoint
  (params (PlayerCharRef :type Actor%20Object%20Reference))
  (Transformation|SetActorLocationAndRotation PlayerCharRef (Transformation|GetWorldLocation (Variables|Default|GetRespawnLocation)) (Transformation|GetWorldRotation (Variables|Default|GetArrow)) false true))