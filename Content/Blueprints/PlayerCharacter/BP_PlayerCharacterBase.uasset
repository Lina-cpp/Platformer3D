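; Base player character Blueprint that handles outfit setup, respawning and the pause menu.
; On begin play it applies the hat from the Game Instance's current outfit.
; The C++-triggered death event moves the player to the gamemode respawn point indexed by the Game Instance's active point, then respawns.
; Pause input toggles the pause widget, disabling or restoring walking movement and updating the Game Instance's paused flag.
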(event Custom|PauseWidgetOff
  (Widget|RemovefromParent (Variables|Default|GetPauseWidget))
  (Variables|Default|SetPauseWidget 0)
  (Pawn|Components|CharacterMovement|SetMovementMode (Variables|Character|GetCharacterMovement) "MOVE_Walking" 0)
  (Variables|/Game/Blueprints/Base/GI_Main.GI_Main_C|SetbIsPaused (CallFunction|GetGI) false))

(event Custom|PauseWidgetON
  (bind _returnvalue (UserInterface|CreateWidget "/Game/Widgets/Game/WBP_PauseMenu.WBP_PauseMenu_C"))
  (bind _output_get (Variables|Default|SetPauseWidget _returnvalue))
  (UserInterface|Viewport|AddtoViewport _output_get 0)
  (Pawn|Components|CharacterMovement|DisableMovement (Variables|Character|GetCharacterMovement))
  (Variables|/Game/Blueprints/Base/GI_Main.GI_Main_C|SetbIsPaused (CallFunction|GetGI) true))

(event Input|EnhancedActionEvents|EnhancedInputActionIA_Pause
  (params (ActionValue :type Boolean) (ElapsedSeconds :type Float%20%28double-precision%29) (TriggeredSeconds :type Float%20%28double-precision%29) (InputAction :type Input%20Action%20Object%20Reference :default "/Game/Blueprints/Inputs/IA_Pause.IA_Pause"))
  (:Started
    (if (not (Variables|/Game/Blueprints/Base/GI_Main.GI_Main_C|GetbIsPaused (CallFunction|GetGI)))
      (CallFunction|PauseWidgetON)
      (else
        (CallFunction|PauseWidgetOff)))))

(event EventBeginPlay
  (Class|CharacterBase|SetClothing (.hat (Variables|/Game/Blueprints/Base/GI_Main.GI_Main_C|GetCurrentOutfit (CallFunction|GetGI)))))

(event EventOnDeath
  ;[0.15 0.15 0.15 0.5] OnDeath (Called in cpp) Get active repawn point and move player there
  (Default|MovePlayertoRespawnPoint (Utilities|Array|Get(acopy) (Variables|/Game/Blueprints/Base/GM_BaseGameMode.GM_BaseGameMode_C|GetRespawnPoints (CallFunction|GetGameplayGamemode)) (Variables|/Game/Blueprints/Base/GI_Main.GI_Main_C|GetActiveRespawnPoint (CallFunction|GetGI))) self)
  (Class|CharacterBase|Respawn))

(fn ConstructionScript)