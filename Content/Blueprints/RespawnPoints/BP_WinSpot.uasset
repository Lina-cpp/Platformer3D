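; Level win trigger that shows the WBP_GameWon screen when a living player character overlaps its box and records the finish time.
; The player name and the widget's times go into an SG_Ranking save slot named after the level, created on first win.
; An existing ranking is re-sorted by total milliseconds via BubbleSortArray and trimmed to MaxIndexesInSaveArray.
; An older insert-by-comparison ranking loop remains in the event graph, unconnected.
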(event OnComponentBeginOverlap(Box)
  (params (OverlappedComponent :type Primitive%20Component%20Object%20Reference) (OtherActor :type Actor%20Object%20Reference) (OtherComp :type Primitive%20Component%20Object%20Reference) (OtherBodyIndex :type Integer) (bFromSweep :type Boolean) (SweepResult :type Hit%20Result%20Structure%20%28by%20ref%29))
  ;[0.15 0.15 0.15 0.5] Check win conditions
  (bind _asbp_player_character_base (Utilities|Casting|CastToBP_PlayerCharacterBase OtherActor))
  (if (not (Variables|/Script/Platformer3D.CharacterBase|GetbIsDead _asbp_player_character_base))
    (bind _returnvalue (UserInterface|CreateWidget "/Game/Widgets/Game/WBP_GameWon.WBP_GameWon_C"))
    (bind _output_get (Variables|Default|SetGameWonWidget _returnvalue))
    (UserInterface|Viewport|AddtoViewport _output_get 0)
    ;[0.15 0.15 0.15 0.5] Save level name and check if savefile for this level already exist
    (bind _returnvalue_2 (Game|GetCurrentLevelName true))
    (bind _output_get_2 (Variables|Default|SetCurrentLevelAndSaveSlotName _returnvalue_2))
    (bind _returnvalue_3 (SaveGame|DoesSaveGameExist _output_get_2))
    (if _returnvalue_3
      (bind _returnvalue_4 (SaveGame|LoadGamefromSlot (Variables|Default|GetCurrentLevelAndSaveSlotName)))
      (bind _assg_ranking (Utilities|Casting|CastToSG_Ranking _returnvalue_4))
      (Utilities|Array|Add (Variables|/Game/Blueprints/GameSave/SG_Ranking.SG_Ranking_C|GetRanking _assg_ranking) (Utilities|Struct|MakeS_RankingVars (Variables|/Game/Blueprints/Base/GI_Main.GI_Main_C|GetPlayerName (CallFunction|GetGI)) (Variables|/Game/Widgets/Game/WBP_GameWon.WBP_GameWon_C|GetElapsedSeconds (Variables|Default|GetGameWonWidget)) (Variables|/Game/Widgets/Game/WBP_GameWon.WBP_GameWon_C|GetTimeInMiliseconds (Variables|Default|GetGameWonWidget)) (Variables|/Game/Widgets/Game/WBP_GameWon.WBP_GameWon_C|GetAll_In_MS (Variables|Default|GetGameWonWidget))))
      (bind _sortedarray (CallFunction|BubbleSortArray (Variables|/Game/Blueprints/GameSave/SG_Ranking.SG_Ranking_C|GetRanking _assg_ranking)))
      (bind _output_get_3 (Variables|/Game/Blueprints/GameSave/SG_Ranking.SG_Ranking_C|SetRanking _assg_ranking _sortedarray))
      (if (> (Utilities|Array|Length _output_get_3) (Variables|Default|GetMaxIndexesInSaveArray))
        (Utilities|Array|RemoveIndex _output_get_3 (Utilities|Array|LastIndex _output_get_3)))
      (bind _returnvalue_5 (SaveGame|SaveGametoSlot _assg_ranking (Variables|Default|GetCurrentLevelAndSaveSlotName)))
      (Development|PrintString (Utilities|String|ToString(Boolean) _returnvalue_5))
      (else
        ;[0.15 0.15 0.15 0.5] Save first record
        (bind _returnvalue_6 (SaveGame|CreateSaveGameObject "/Game/Blueprints/GameSave/SG_Ranking.SG_Ranking_C"))
        (Utilities|Array|Add (Variables|/Game/Blueprints/GameSave/SG_Ranking.SG_Ranking_C|GetRanking _returnvalue_6) (Utilities|Struct|MakeS_RankingVars (Variables|/Game/Blueprints/Base/GI_Main.GI_Main_C|GetPlayerName (CallFunction|GetGI)) (Variables|/Game/Widgets/Game/WBP_GameWon.WBP_GameWon_C|GetElapsedSeconds (Variables|Default|GetGameWonWidget)) (Variables|/Game/Widgets/Game/WBP_GameWon.WBP_GameWon_C|GetTimeInMiliseconds (Variables|Default|GetGameWonWidget)) (Variables|/Game/Widgets/Game/WBP_GameWon.WBP_GameWon_C|GetAll_In_MS (Variables|Default|GetGameWonWidget))))
        (SaveGame|SaveGametoSlot _returnvalue_6 (Variables|Default|GetCurrentLevelAndSaveSlotName))))))

(event Custom|CallBreakLoop
  (bind _rankingref (Variables|Default|GetRankingRef))
  (bind _gamewonwidget (Variables|Default|GetGameWonWidget))
  (bind _rankingref_2 (Variables|Default|GetRankingRef))
  (bind _gamewonwidget_2 (Variables|Default|GetGameWonWidget))
  (bind _gamewonwidget_3 (Variables|Default|GetGameWonWidget))
  (bind _ranking (Variables|/Game/Blueprints/GameSave/SG_Ranking.SG_Ranking_C|GetRanking _rankingref_2))
  (bind _ranking_2 (Variables|/Game/Blueprints/GameSave/SG_Ranking.SG_Ranking_C|GetRanking _rankingref))
  ;[0.15 0.15 0.15 0.5] Kinda working
  (Utilities|Array|ForEachLoopwithBreak (Variables|/Game/Blueprints/GameSave/SG_Ranking.SG_Ranking_C|GetRanking (stale _output_get))) ; enters at Break
)

(event EventBeginPlay
  (|CallParentFunction) ; This node is disabled and will not be called.\nDrag off pins to build functionality.
)

(event Collision|EventActorBeginOverlap
  (params (OtherActor :type Actor%20Object%20Reference))
  (|CallParentFunction OtherActor) ; This node is disabled and will not be called.\nDrag off pins to build functionality.
)

(event EventTick
  (params (DeltaSeconds :type Float%20%28single-precision%29))
  (|CallParentFunction DeltaSeconds) ; This node is disabled and will not be called.\nDrag off pins to build functionality.
)

(fn ConstructionScript
  (|CallParentFunction))

(fn RemoveAdditionIndexes
  (params (RankingArray :type Array%20of%20S%20Ranking%20Vars%20Structures))
  (if (> (Utilities|Array|Length RankingArray) (Variables|Default|GetMaxIndexesInSaveArray))
    (Utilities|Array|RemoveIndex RankingArray (Utilities|Array|LastIndex RankingArray)))
  (return))

(fn BubbleSortArray
  (params (RankingArray :type Array%20of%20S%20Ranking%20Vars%20Structures))
  (bind _returnvalue (Utilities|Array|LastIndex RankingArray))
  (for _index (range 0 _returnvalue)
    (for _index_2 (range _index _returnvalue)
      (if (> (.all_in_ms (Utilities|Array|Get(acopy) RankingArray _index)) (.all_in_ms (Utilities|Array|Get(acopy) RankingArray _index_2)))
        (Utilities|Array|Swap RankingArray _index_2 _index))))
  (return RankingArray))